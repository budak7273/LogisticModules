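; Parent attachment class for power suit logistic modules, holding the shared power, range, toggle and desired-item logic, with overridable hooks for item deltas and status text.
; On authority, power suit stat updates trigger a delayed recalculation from mod config and installed amplifier, stabilizer, range and synchronizer upgrades.
; Power draw decays on a timed tick.
; Locally controlled clients forward toggle and desired-item edits to the server through replicated events.
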(event `self.AttachmentInstalled`
  (params (Item :type "InventoryItem Structure"))
  (`parent.AttachmentInstalled` Item)
  (`/Engine/EditorBlueprintResources/ActorMacros.Switch Has Authority`
    (:`Authority`
      (add `PowerSuit.OnPowerSuitStatUpdate` (`EquipmentModuleComponent.EquipmentParent` (`self.ParentModule`)) (delegate `OnPowerSuitStatUpdate`))
      (`self.OnPowerSuitStatUpdate` 0))))

(event `OnPowerSuitStatUpdate`
  (params (Type :type Integer))
  (`KismetSystemLibrary.Delay` 0.2) ; Prevent recalc spam
  (`self.SetupDefaults`)
  (`BlueprintLoggingLibrary.LogDisplay` "Logistic Parent Setup Defaults"))

(event `self.AttachmentUnInstalled`
  (`parent.AttachmentUnInstalled`)
  (`/Engine/EditorBlueprintResources/ActorMacros.Switch Has Authority`
    (:`Authority`
      (remove `PowerSuit.OnPowerSuitStatUpdate` (`EquipmentModuleComponent.EquipmentParent` (`self.ParentModule`)) (delegate `OnPowerSuitStatUpdate`)))))

(event `self.AttachmentTick`
  (params (DeltaTime :type "Float (single-precision)"))
  (`parent.AttachmentTick` DeltaTime)
  (`/Engine/EditorBlueprintResources/ActorMacros.Switch Has Authority`
    (:`Authority`
      (`KismetSystemLibrary.Delay` (`self.PowerDecayInterval`))
      (`self.Update Power Consumption`))))

(event `Set Toggle Switch`
  (params (`UI Toggle Switch Enabled` :type Boolean))
  (bind _returnvalue (`KismetStringLibrary.Conv_BoolToString` `UI Toggle Switch Enabled`))
  (`/Engine/EditorBlueprintResources/ActorMacros.Switch Has Authority`
    (:`Authority`
      (set `self.UI Toggle Switch Enabled` `UI Toggle Switch Enabled`)
      (`BlueprintLoggingLibrary.LogVerbose` (`KismetStringLibrary.Concat_StrStr` "Authority Set Toggle Switch " _returnvalue)))
    (:`Remote`
      (if (`FGBlueprintFunctionLibrary.IsLocallyHumanControlled` (`self.Instigator`))
        (`self.Remote_SetToggleSwitch` `UI Toggle Switch Enabled`)
        (`BlueprintLoggingLibrary.LogVerbose` (`KismetStringLibrary.Concat_StrStr` "REMOTE REQUEST Set Toggle Switch " _returnvalue))
        (else
          (`BlueprintLoggingLibrary.LogVerbose` "Remote not Locally Controlled, doing nothing for toggle switch"))))))

(event `Remote_SetToggleSwitch`
  (params (`UI Toggle Switch Enabled` :type Boolean))
  (bind _output_get (set `self.UI Toggle Switch Enabled` `UI Toggle Switch Enabled`))
  (`BlueprintLoggingLibrary.LogVerbose` (`KismetStringLibrary.Concat_StrStr` "REP Set Toggle Switch " (`KismetStringLibrary.Conv_BoolToString` _output_get))))

(event `Remote_SetItem`
  (params (Class :type "Object Class Reference") (Amount :type Integer) (`Remove at 0` :type Boolean))
  (`BlueprintLoggingLibrary.LogVerbose` (`KismetStringLibrary.Concat_StrStr` "REP Set Item " (`KismetSystemLibrary.GetClassDisplayName` Class) " x " (`KismetStringLibrary.Conv_IntToString` Amount)))
  (`self.Set Desired Item` Class Amount `Remove at 0`))

(event `Remote_ClearDesiredItems`
  (`BlueprintLoggingLibrary.LogVerbose` "REP Clear Desired Items")
  (`self.ClearDesiredItems`))

(event `Remote_ReplaceAllDesiredItems`
  (params (UserDesiredItems :type "Array of ItemAmount Structure"))
  (`BlueprintLoggingLibrary.LogVerbose` (`KismetStringLibrary.Concat_StrStr` "REP ReplaceDesiredItems with length " (`KismetStringLibrary.Conv_IntToString` (`KismetArrayLibrary.Array_Length` UserDesiredItems))))
  (set `self.UserDesiredItems` UserDesiredItems))

(fn `ClearDesiredItems`
  (`/Engine/EditorBlueprintResources/ActorMacros.Switch Has Authority`
    (:`Authority`
      (`KismetArrayLibrary.Array_Clear` (`self.UserDesiredItems`)))
    (:`Remote`
      (if (`FGBlueprintFunctionLibrary.IsLocallyHumanControlled` (`self.Instigator`))
        (`self.Remote_ClearDesiredItems`)))))

(fn `Get Message for Display`
  (returns (ReturnValue :type Text))
  (bind _returnvalue (- (`KismetMathLibrary.UtcNow`) (`self.LastMessageTime`)))
  (bind _message (`self.Module Specific Custom Message`))
  (return (select `bool` (< _returnvalue (`KismetMathLibrary.MakeTimespan` 0 0 0 3)) :`false` (select `bool` (`self.Busy Operating`) :`false` (select `bool` (`self.UI Toggle Switch Enabled`) :`false` "Status: Disabled by User" :`true` _message) :`true` "Status: Busy") :`true` (`|FormatText` "{StatusMessage} ({TimeLeft} sec)" (`self.StatusMessage`) (`KismetTextLibrary.Conv_DoubleToText` (- (`KismetMathLibrary.Conv_IntToDouble` 3) (`KismetMathLibrary.GetTotalSeconds` _returnvalue)) "HalfToEven" false true 1 324 1 1)))))

(fn `GetDeltaPowerConsumption`
  (params (DeltaTime :type "Float (double-precision)"))
  (returns (ReturnValue :type "Float (double-precision)"))
  (return (+ (`self.CurrentPowerConsumption`) (`KismetMathLibrary.SelectFloat` (* (`self.Passive Power Usage MW`) (`self.Cached Passive Power Cost Mult`)) 0.0 (`self.UI Toggle Switch Enabled`)))))

(fn `Module Specific Calc Delta Items`
  (returns (`Item Delta` :type "Map of FGItemDescriptor Class Reference to Integer"))
  (locals (`Build Delta` :type "Map of FGItemDescriptor Class Reference to Integer"))
  ;[1 1 1] Can be implemented per module. Default is to put all >0 Desired in the records
  (for _array_element (`self.UserDesiredItems`)
    (bind (_itemclass _amount) (break `ItemAmount` _array_element))
    (if (> _amount 0)
      (`BlueprintMapLibrary.Map_Add` (`local.Build Delta`) _itemclass _amount)
      (`/LogisticModules/Blueprints/Lib_LogisticModules.Log Item Search` false (`KismetTextLibrary.Conv_TextToString` (`FGItemDescriptor.GetItemName` _itemclass)) (`KismetStringLibrary.Concat_StrStr` " x " (`KismetStringLibrary.Conv_IntToString` _amount)))))
  (return (`local.Build Delta`)))

(fn `Module Specific Custom Message`
  (returns (Message :type Text))
  (return "Status: Ready"))

(fn `Post Status Message`
  (params (UserMessage :type Text))
  (set `self.StatusMessage` UserMessage)
  (set `self.LastMessageTime` (`KismetMathLibrary.UtcNow`)))

(fn `Set Desired Item`
  (params (Class :type "Object Class Reference") (Amount :type Integer) (RemoveAt0 :type Boolean))
  (locals (Found :type Boolean) (`Remove at 0` :type Boolean))
  (set `local.Remove at 0` RemoveAt0)
  (bind _asfgitem_descriptor (castclass `FGItemDescriptor` Class))
  (`/Engine/EditorBlueprintResources/ActorMacros.Switch Has Authority`
    (:`Authority`
      (`BlueprintLoggingLibrary.LogVerbose` (`KismetStringLibrary.Concat_StrStr` "Authority Set Item " (`KismetSystemLibrary.GetClassDisplayName` _asfgitem_descriptor) " x " (`KismetStringLibrary.Conv_IntToString` Amount)))
      (for (_array_element _array_index) (`self.UserDesiredItems`) :!label _label
        (bind (_itemclass _amount) (break `ItemAmount` _array_element))
        (if (== _itemclass _asfgitem_descriptor)
          (set `local.Found` true)
          (if (== Amount 0)
            (if (`local.Remove at 0`)
              (`KismetArrayLibrary.Array_Remove` (`self.UserDesiredItems`) _array_index)
              (break))
            (elif (not (== _amount Amount))
              (`KismetArrayLibrary.Array_Set` (`self.UserDesiredItems`) _array_index (make `ItemAmount` _asfgitem_descriptor Amount))
              (break)))))
      (if (not (`local.Found`))
        (`KismetArrayLibrary.Array_Add` (`self.UserDesiredItems`) (make `ItemAmount` _asfgitem_descriptor Amount))))
    (:`Remote`
      (if (`FGBlueprintFunctionLibrary.IsLocallyHumanControlled` (`self.Instigator`))
        (`self.Remote_SetItem` _asfgitem_descriptor Amount (`local.Remove at 0`))
        (`BlueprintLoggingLibrary.LogVerbose` (`KismetStringLibrary.Concat_StrStr` "REMOTE REQUEST Set Item but also executing locally " (`KismetSystemLibrary.GetClassDisplayName` _asfgitem_descriptor) " x " (`KismetStringLibrary.Conv_IntToString` Amount)))
        (goto _label)
        (else
          (`BlueprintLoggingLibrary.LogVerbose` "Remote not Locally Controlled, doing nothing for Set Item"))))))

(fn `SetupDefaults`
  (bind _parentmodule (`self.ParentModule`))
  (bind _asbp_config_property_section (cast `/SML/ModList/Properties/BP_ConfigPropertySection` (`RuntimeBlueprintFunctionLibrary.Conv_ConfigPropertySectionToConfigProperty` (cast `/SML/ModList/Properties/BP_ConfigPropertySection` (`RuntimeBlueprintFunctionLibrary.Conv_ModConfigurationToConfigProperty` "/LogisticModules/LogisticModules_Configuration.LogisticModules_Configuration_C") :!pure true) "Balance") :!pure true))
  (set `self.Cached Passive Power Cost Mult` (`RuntimeBlueprintFunctionLibrary.Conv_ConfigPropertyToFloat` (`RuntimeBlueprintFunctionLibrary.Conv_ConfigPropertySectionToConfigProperty` _asbp_config_property_section "PassivePowerUsageMult")))
  (set `self.Cached Per Task Power Cost Mult` (`RuntimeBlueprintFunctionLibrary.Conv_ConfigPropertyToFloat` (`RuntimeBlueprintFunctionLibrary.Conv_ConfigPropertySectionToConfigProperty` _asbp_config_property_section "PerTaskPowerUsageMult")))
  (set `self.BuildingRecordsUpdateInterval` (`RuntimeBlueprintFunctionLibrary.Conv_ConfigPropertyToFloat` (`RuntimeBlueprintFunctionLibrary.Conv_ConfigPropertySectionToConfigProperty` _asbp_config_property_section "AutoBuildingSearchIntervalSeconds")))
  (set `self.AutomaticOperationIntervalSeconds` (`RuntimeBlueprintFunctionLibrary.Conv_ConfigPropertyToFloat` (`RuntimeBlueprintFunctionLibrary.Conv_ConfigPropertySectionToConfigProperty` _asbp_config_property_section "AutoItemMovementIntervalSeconds")))
  (set `self.PowerConsumptionMax` (`self.Base MaxPowerCost MW`))
  (set `self.RangeIncrease Mult` 1.0)
  (set `self.SynchronizerInstalled` false)
  (set `self.StabilizerInstalled` false)
  (set `self.AmplifierInstalled` false)
  (for _array_element (`FGInventoryComponent.GetInventoryStacks` (`EquipmentModuleComponent.nInventory` (`self.ParentModule`)))
    (bind _out_itemclass (`FGInventoryLibrary.BreakInventoryItem` (`.out_item` (`FGInventoryLibrary.BreakInventoryStack` _array_element))))
    (castclass `/LogisticModules/Items/Passive/LogisticPowerAmplifier/Module_LogisticPowerAmplifier` _out_itemclass
      (:`then`
        (set `self.AmplifierInstalled` true))
      (:`CastFailed`
        (castclass `/LogisticModules/Items/Passive/LogisticPowerStablizier/Module_LogisticPowerStablizier` _out_itemclass
          (:`then`
            (set `self.StabilizerInstalled` true))
          (:`CastFailed`
            (castclass `/LogisticModules/Items/Passive/LogisticRangeIncreaseMK1/Module_LogisticRangeIncreaseMK1` _out_itemclass
              (:`then`
                (`/Engine/EditorBlueprintResources/StandardMacros.IncrementFloat` (`self.RangeIncrease Mult`)))
              (:`CastFailed`
                (castclass `/LogisticModules/Items/Passive/LogisticRangeIncreaseMk2/Module_LogisticRangeIncreaseMK2` _out_itemclass
                  (:`then`
                    (set `self.RangeIncrease Mult` (+ (`self.RangeIncrease Mult`) 1.3)))
                  (:`CastFailed`
                    (castclass `/LogisticModules/Items/Passive/LogisticSynchronizer/Module_LogisticSynchronizer` _out_itemclass)
                    (set `self.SynchronizerInstalled` true))))))))))
  (`|ExecutionSequence`
    (:`then_0`
      (set `self.RangeCentimeters` (* (`self.RangeIncrease Mult`) (`self.Base Range Cm`))))
    (:`then_1`
      (set `self.PowerDecayInterval` (* (+ (`KismetMathLibrary.Conv_BoolToInt` (`self.StabilizerInstalled`)) 1) (`self.Base PowerDecayInterval Seconds`)))
      (set `self.PowerCostPerTask` (* (`self.Cached Per Task Power Cost Mult`) (select `bool` (`self.StabilizerInstalled`) :`false` (`self.Default PowerCostPerTask MW`) :`true` (`self.Stabilized PowerCostPerTask MW`)))))
    (:`then_2`
      ;[1 1 1] Amplifier
      (if (`self.AmplifierInstalled`)
        (set `self.PowerDecayInterval` (`KismetMathLibrary.SafeDivide` (`self.PowerDecayInterval`) (`self.ValueOrOneIfZero` (`.Modifier` (break `ModMultProperty` (`EquipmentModuleComponent.GetNamedPropertySafe` _parentmodule "LogisticDecayIntervalDivideBy"))))))
        (set `self.PowerCostPerTask` (* (`self.PowerCostPerTask`) (`self.ValueOrOneIfZero` (`.Modifier` (break `ModMultProperty` (`EquipmentModuleComponent.GetNamedPropertySafe` _parentmodule "LogisticCostPerTaskMultBy"))))))))
    (:`then_3`
      ;[1 1 1] Synchronizer
      (if (`self.SynchronizerInstalled`)
        (set `self.PowerConsumptionMax` (`KismetMathLibrary.FClamp` (- (`self.PowerConsumptionMax`) (`.Modifier` (break `ModMultProperty` (`EquipmentModuleComponent.GetNamedPropertySafe` (`self.ParentModule`) "LogisticSyncMaxPowerReduction")))) 0.0 (`self.PowerConsumptionMax`)))))))

(fn `ShouldSave`
  (returns (ReturnValue :type Boolean))
  (return true))

(fn `TODEL Calculate Needed Items from Desired`
  (params (`Exclude Active Transfers` :type Boolean) (`Optional Inventory Exclude Contents Of` :type "FGInventoryComponent Object Reference"))
  (returns (`Item Delta` :type "Map of FGItemDescriptor Class Reference to Integer"))
  (locals (BuildNeeded :type "Map of FGItemDescriptor Class Reference to Integer"))
  (bind _buildneeded (`local.BuildNeeded`))
  (bind _buildneeded_2 (`local.BuildNeeded`))
  (for _array_element (`self.UserDesiredItems`)
    (bind (_itemclass _amount) (break `ItemAmount` _array_element))
    ;[1 1 1] Put all non-zero Desired in the records
    (if (> _amount 0)
      (`BlueprintMapLibrary.Map_Add` (`local.BuildNeeded`) _itemclass _amount)
      (`/LogisticModules/Blueprints/Lib_LogisticModules.Log Item Search` false (`KismetTextLibrary.Conv_TextToString` (`FGItemDescriptor.GetItemName` _itemclass)) (`KismetStringLibrary.Concat_StrStr` " x " (`KismetStringLibrary.Conv_IntToString` _amount)))))
  (if `Exclude Active Transfers`
    ;[1 1 1] Leave out items currently being transferred (used by Subscribe)
    (bind _keys (`BlueprintMapLibrary.Map_Keys` (`self.Transfer to ItemAmount`)))
    (for _array_element_2 _keys
      (`/Engine/EditorBlueprintResources/StandardMacros.IsValid` _array_element_2
        (:`Is Valid`
          (bind (_itemclass_2 _amount_2) (break `ItemAmount` (`BlueprintMapLibrary.Map_Find` (`self.Transfer to ItemAmount`) _array_element_2)))
          (bind _returnvalue (- (`BlueprintMapLibrary.Map_Find` (`local.BuildNeeded`) _itemclass_2) _amount_2))
          (if (> _returnvalue 0)
            (`BlueprintMapLibrary.Map_Add` _buildneeded _itemclass_2 _returnvalue)
            (else
              (`BlueprintMapLibrary.Map_Remove` _buildneeded _itemclass_2))))
        (:`Is Not Valid`
          (`BlueprintMapLibrary.Map_Remove` (`self.Transfer to ItemAmount`) _array_element_2)
          (`BlueprintLoggingLibrary.LogWarning` "Cleaned up a transfer that no longer had an active SendItem")))))
  (if (`KismetSystemLibrary.IsValid` `Optional Inventory Exclude Contents Of`)
    ;[1 1 1] Exclude items already present in an inventory (used by Disperse)
    (bind _keys_2 (`BlueprintMapLibrary.Map_Keys` (`local.BuildNeeded`)))
    (for _array_element_3 _keys_2
      (bind _returnvalue_2 (- (`BlueprintMapLibrary.Map_Find` (`local.BuildNeeded`) _array_element_3) (`FGInventoryComponent.GetNumItems` `Optional Inventory Exclude Contents Of` _array_element_3)))
      (if (> _returnvalue_2 0)
        (`BlueprintMapLibrary.Map_Add` _buildneeded_2 _array_element_3 _returnvalue_2)
        (else
          (`BlueprintMapLibrary.Map_Remove` _buildneeded_2 _array_element_3)))))
  (return (`local.BuildNeeded`)))

(fn `Update Power Consumption`
  (bind _currentpowerconsumption (`self.CurrentPowerConsumption`))
  (if (<= _currentpowerconsumption 0.25)
    (set `self.CurrentPowerConsumption` 0.0)
    (else
      (set `self.CurrentPowerConsumption` (`KismetMathLibrary.FClamp` (- _currentpowerconsumption (`KismetMathLibrary.FClamp` (/ (- (`self.PowerConsumptionMax`) _currentpowerconsumption) 2.0) 5.0 10.0)) 0.0 (`self.PowerConsumptionMax`))))))

(fn `UserConstructionScript`)
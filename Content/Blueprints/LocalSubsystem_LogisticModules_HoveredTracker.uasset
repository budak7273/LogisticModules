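; Local subsystem for Logistic Modules that tracks the last hovered item and adds a disperse keybind hint to item tooltips.
; On BeginPlay it hooks Widget_Tooltip's Construct, working around SML tooltip providers lacking world context.
; If the config option is on and a cached suit disperser exists, it records the item and injects Widget_DisperseKeybind into the tooltip's canvas.
; The older root-instance reference handoff and debug logging are disconnected.
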(event `On Widget Tooltip Construct`
  (params (Object :type "Object Object Reference"))
  ;[1 1 1] SML Tooltip Providers don't have world context so have to do this ourselves
  (if (`RuntimeBlueprintFunctionLibrary.Conv_ConfigPropertyToBool` (`RuntimeBlueprintFunctionLibrary.Conv_ConfigPropertySectionToConfigProperty` (cast `/SML/ModList/Properties/BP_ConfigPropertySection` (`RuntimeBlueprintFunctionLibrary.Conv_ConfigPropertySectionToConfigProperty` (cast `/SML/ModList/Properties/BP_ConfigPropertySection` (`RuntimeBlueprintFunctionLibrary.Conv_ModConfigurationToConfigProperty` "/LogisticModules/LogisticModules_Configuration.LogisticModules_Configuration_C") :!pure true) "Interface") :!pure true) "DisperserTooltip"))
    (`/Engine/EditorBlueprintResources/StandardMacros.IsValid` (`self.Cached Disperser Attachment`) ; Don't add stuff in unless we have a disperser installed in a suit
      (:`Is Valid`
        (bind _aswidget_tooltip (cast `/Game/FactoryGame/Interface/UI/InGame/Tooltip/Widget_Tooltip` Object))
        (bind _output_get (set `self.LastHoveredItemAmount` (`/Game/FactoryGame/Interface/UI/InGame/Tooltip/Widget_Tooltip.mItemDescriptor` _aswidget_tooltip)))
        (bind _ascanvas_panel (cast `CanvasPanel` (`Widget.GetParent` (`/Game/FactoryGame/Interface/UI/InGame/Tooltip/Widget_Tooltip.mSizeBox` _aswidget_tooltip)))
          (:`then`
            (bind _returnvalue (`|CreateWidget` "/LogisticModules/Items/Active/LogisticDisperse/Widget_DisperseKeybind.Widget_DisperseKeybind_C" null _output_get))
            (bind _output_get_2 (set `self.Cached Tooltip Widget` _returnvalue))
            (bind _returnvalue_2 (`CanvasPanel.AddChildToCanvas` _ascanvas_panel _output_get_2))
            ;[1 1 1] Measured from adding it in the editor to Widget_Tooltip
            (`CanvasPanelSlot.SetPosition` _returnvalue_2 (4.0 -40.0))
            (`CanvasPanelSlot.SetSize` _returnvalue_2 (240.0 30.0))
            (`CanvasPanelSlot.SetAutoSize` _returnvalue_2 true))
          (:`CastFailed`
            (`BlueprintLoggingLibrary.LogError` "Tooltip size box parent wasn't canvas panel?")))))))

(event `self.ReceiveBeginPlay`
  (`parent.ReceiveBeginPlay`)
  (`RuntimeBlueprintFunctionLibrary.BindOnBPFunction` "/Game/FactoryGame/Interface/UI/InGame/Tooltip/Widget_Tooltip.Widget_Tooltip_C" (delegate `On Widget Tooltip Construct`) "Construct"))

(event `self.ReceiveEndPlay`
  (params (EndPlayReason :type "EEndPlayReason Enum" :default "Destroyed"))
  (`parent.ReceiveEndPlay` EndPlayReason))

(event `self.ReceiveTick`
  (params (DeltaSeconds :type "Float (single-precision)")))

(fn `UserConstructionScript`)
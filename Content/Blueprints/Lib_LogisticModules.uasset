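; Helper function library for the Logistic Modules mod, covering config reads, item search logging and actor outlining.
; Config getters walk nested mod configuration sections for interface click request sizes and a debug toggle that gates item search warning and verbose logs.
; Outlining finds FGOutlineComponent on the first player controller or its pawn, then adds proxy outlines for instanced spline meshes, skipping legs and feet, alongside a multi-actor outline marked as possibly broken.
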(fn `Do Item Search Logging?`
  (returns (Enabled :type Boolean))
  (return (`RuntimeBlueprintFunctionLibrary.Conv_ConfigPropertyToBool` (`RuntimeBlueprintFunctionLibrary.Conv_ConfigPropertySectionToConfigProperty` (cast `/SML/Interface/UI/Menu/Mods/ConfigProperties/BP_ConfigPropertySection` (`RuntimeBlueprintFunctionLibrary.Conv_ConfigPropertySectionToConfigProperty` (cast `/SML/Interface/UI/Menu/Mods/ConfigProperties/BP_ConfigPropertySection` (`RuntimeBlueprintFunctionLibrary.Conv_ModConfigurationToConfigProperty` "/LogisticModules/LogisticModules_Configuration.LogisticModules_Configuration_C") :!pure true) "Debugging") :!pure true) "ItemSearchLogging"))))

(fn `Get Config Click Request Size`
  (params (`Interface section Sub Key` :type String))
  (returns (ReturnValue :type Integer))
  (return (`RuntimeBlueprintFunctionLibrary.Conv_ConfigPropertyToInteger` (`RuntimeBlueprintFunctionLibrary.Conv_ConfigPropertySectionToConfigProperty` (cast `/SML/Interface/UI/Menu/Mods/ConfigProperties/BP_ConfigPropertySection` (`RuntimeBlueprintFunctionLibrary.Conv_ConfigPropertySectionToConfigProperty` (cast `/SML/Interface/UI/Menu/Mods/ConfigProperties/BP_ConfigPropertySection` (`RuntimeBlueprintFunctionLibrary.Conv_ModConfigurationToConfigProperty` "/LogisticModules/LogisticModules_Configuration.LogisticModules_Configuration_C") :!pure true) "Interface") :!pure true) `Interface section Sub Key`))))

(fn `Get Outline Component`
  (params (WorldContextObject :type "Object Object Reference"))
  (returns (ReturnValue :type "FGOutlineComponent Object Reference"))
  (bind _returnvalue (`GameplayStatics.GetPlayerController` WorldContextObject))
  (bind _returnvalue_2 (`Actor.GetComponentByClass` _returnvalue "/Script/FactoryGame.FGOutlineComponent"))
  (return (select `bool` (`KismetSystemLibrary.IsValid` _returnvalue_2) :`false` (`Actor.GetComponentByClass` (`Controller.K2_GetPawn` _returnvalue) "/Script/FactoryGame.FGOutlineComponent") :`true` _returnvalue_2)))

(fn `Log Item Search`
  (params (`Is Warning` :type Boolean :default true) (Str1 :type String) (Str2 :type String))
  (bind _returnvalue (`KismetStringLibrary.Concat_StrStr` Str1 Str2))
  (if (`self.Do Item Search Logging?` null)
    (if `Is Warning`
      (`BlueprintLoggingLibrary.LogWarning` _returnvalue)
      (else
        (`BlueprintLoggingLibrary.LogVerbose` _returnvalue)))))

(fn `Show Outline on Actors`
  (params (color :type "EOutlineColor Enum" :default "OC_NONE") (ActorsToOutline :type "Array of Actor Object Reference"))
  (locals (OutlineComponent :type "FGOutlineComponent Object Reference") (Components :type "Array of InstancedSplineMeshComponent Object Reference"))
  (bind _output (`|GetArrayItem` ActorsToOutline))
  (bind _output_get (set `local.OutlineComponent` (`self.Get Outline Component` _output _output)))
  (`FGOutlineComponent.ShowMultiActorOutline` _output_get ActorsToOutline color) ; TODO U6 this doesn't seem to be working, ben said would fix?
  (for _array_element ActorsToOutline
    (bind _output_get_2 (set `local.Components` (`Actor.K2_GetComponentsByClass` _array_element "/Script/InstancedSplinesComponent.InstancedSplineMeshComponent")))
    (for _array_element_2 _output_get_2
      (bind _returnvalue (`KismetSystemLibrary.GetDisplayName` _array_element_2))
      (if (not (or (`KismetStringLibrary.Contains` _returnvalue "Leg") (`KismetStringLibrary.Contains` _returnvalue "Foot")))
        (`FGOutlineComponent.ShowProxyOutline` (`local.OutlineComponent`) (`StaticMeshComponent.StaticMesh` _array_element_2) (`SceneComponent.K2_GetComponentToWorld` _array_element_2) color)))))
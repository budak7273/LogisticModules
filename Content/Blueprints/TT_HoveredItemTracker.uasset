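; TT_HoveredItemTracker is a tooltip provider that records the hovered inventory stack for the LogisticModules mod.
; Lacking world context, it reaches the tracker subsystem through a reference on the LogisticModules game instance module and sets its last hovered stack.
; It creates and caches a disperse keybind widget when a disperser attachment is cached, with an uncached fallback widget if lookup fails.
; The item description is empty, and TODOs mark the widget logic as old.
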(fn `CreateDescriptionWidget`
  (params (OwningPlayer :type "PlayerController Object Reference") (InventoryStack :type "InventoryStack Structure (by ref)"))
  (returns (ReturnValue :type "Widget Object Reference"))
  (bind _returnvalue (subsystem `GameInstanceModuleManager`))
  (bind _returnvalue_2 (`GameInstanceModuleManager.FindModule` _returnvalue "LogisticModules"))
  ;[1 1 1] TODO all old
  (`/Engine/EditorBlueprintResources/StandardMacros.IsValid` _returnvalue
    (:`Is Valid`
      (bind _asroot_instance_logistic_modules (cast `/LogisticModules/RootInstance_LogisticModules` _returnvalue_2)
        (:`then`
          (bind _subsystem_reference_for_tooltip_provider (`/LogisticModules/RootInstance_LogisticModules.Subsystem Reference for Tooltip Provider` _asroot_instance_logistic_modules))
          (`/Engine/EditorBlueprintResources/StandardMacros.IsValid` _subsystem_reference_for_tooltip_provider
            (:`Is Valid`
              (set `/LogisticModules/Blueprints/LocalSubsystem_LogisticModules_HoveredTracker.LastHoveredItemStack` InventoryStack _subsystem_reference_for_tooltip_provider)
              (`/Engine/EditorBlueprintResources/StandardMacros.IsValid` (`/LogisticModules/Blueprints/LocalSubsystem_LogisticModules_HoveredTracker.Cached Disperser Attachment` _subsystem_reference_for_tooltip_provider)
                (:`Is Valid`
                  (bind _returnvalue_3 (`|CreateWidget` "/LogisticModules/Items/Active/LogisticDisperse/Widget_DisperseKeybind.Widget_DisperseKeybind_C"))
                  (bind _output_get (set `/LogisticModules/Blueprints/LocalSubsystem_LogisticModules_HoveredTracker.Cached Tooltip Widget` _returnvalue_3 _subsystem_reference_for_tooltip_provider))
                  (return _output_get))
                (:`Is Not Valid`
                  (`BlueprintLoggingLibrary.LogVerbose` "No cached disperser yet")
                  (return null))))
            (:`Is Not Valid`
              _)))
        (:`CastFailed`
          (`BlueprintLoggingLibrary.LogError` (`KismetStringLibrary.Concat_StrStr` "Could not find logistic instance module? was: " (`KismetSystemLibrary.GetDisplayName` _returnvalue_2)) :!label _label))))
    (:`Is Not Valid`
      (`BlueprintLoggingLibrary.LogError` "Game Instance Module Manager is invalid?")
      (goto _label)))
  (`BlueprintLoggingLibrary.LogVerbose` "HoveredTracker subsystem not ready yet?")
  (bind _returnvalue_4 (`|CreateWidget` "/LogisticModules/Items/Active/LogisticDisperse/Widget_DisperseKeybind.Widget_DisperseKeybind_C"))
  (return _returnvalue_4))

(fn `GetItemDescription`
  (params (OwningPlayer :type "PlayerController Object Reference") (InventoryStack :type "InventoryStack Structure (by ref)"))
  (returns (ReturnValue :type Text))
  (return ""))

(fn `UserConstructionScript`)